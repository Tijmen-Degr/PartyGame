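; BP_Rotator is a component that continuously spins either itself or its owner's root component.
; On BeginPlay it picks that target, builds a rotation step from the axes and speed, and can wait a random delay before starting a looping timer.
; The timer drives the local rotation in fixed steps at the update interval, with Tick left empty.
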(event `self.ReceiveTick`
  (params (DeltaSeconds :type "Float (single-precision)")))

(event `self.ReceiveBeginPlay`
  (bind (_returnvalue_x _returnvalue_y _returnvalue_z) (`KismetMathLibrary.BreakVector` (* (`self.Axes`) (* (`self.RotationSpeed`) -2.0))))
  (bind _output_get (set `self.DeltaRotator` (`KismetMathLibrary.MakeRotator` _returnvalue_x _returnvalue_y _returnvalue_z)))
  (set `self.Target` (select `bool` (`self.ApplyToSefl`) :`false` (`Actor.RootComponent` (`self.GetOwner`)) :`true` self :!type "SceneComponent Object Reference"))
  (if (`self.UseRandomInitiaslDelay`)
    (`KismetSystemLibrary.Delay` (`KismetMathLibrary.RandomFloatInRange` 0.0 (`self.RandomInitialDelay`))))
  (`KismetSystemLibrary.K2_SetTimerDelegate` (`|CreateDelegate` :!event `OnUpdate`) (`self.UpdateTime`) true))

(event `OnUpdate`
  (`self.K2_AddLocalRotation` (`self.Target`) (`self.DeltaRotator`) false false))