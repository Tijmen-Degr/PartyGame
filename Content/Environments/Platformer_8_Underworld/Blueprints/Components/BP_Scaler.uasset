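; BP_Scaler is a component in the Underworld platformer environment that animates a target's world scale back and forth.
; On BeginPlay it stores the current world scale and the configured TargetScale as endpoints.
; Each update eases between them using an alpha, a selectable easing function and an exponent.
; At each period end it swaps the endpoints, so the scaling reverses.
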(event `self.ReceiveBeginPlay`
  (`parent.ReceiveBeginPlay`)
  (set `self.ScaleB` (`self.TargetScale`))
  (set `self.ScaleA` (`self.K2_GetComponentScale`)))

(event `self.OnUpdate`
  (`self.SetWorldScale3D` (`self.Target`) (`|EaseFunction` (`self.Function`) (`self.GetAlpha`) (`self.ScaleA`) (`self.ScaleB`) (`self.Exponent`))))

(event `self.OnPeriodEnd`
  (`/Game/Environments/Platformer_8_Underworld/Blueprints/Components/BML_Platformer.Swap` (`self.ScaleA`) (`self.ScaleB`)))