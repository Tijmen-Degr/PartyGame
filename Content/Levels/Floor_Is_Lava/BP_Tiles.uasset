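; BP_Tiles is a stone tile actor for the Floor Is Lava level that shakes and then removes itself.
; The construction script applies the StoneMesh variable to its static mesh.
; The Shake event plays a rock sound and runs a timeline that adds a vertical local offset to the mesh on each update.
; When the timeline finishes, it disables the mesh's collision and destroys the actor.
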(event `Shake`
  (`GameplayStatics.PlaySound2D` "/Game/Levels/Floor_Is_Lava/Rock_Shake.Rock_Shake" 1.5 1.0 0.0 null null)
  (bind (_direction _float) (`Timeline|Timeline_0`)
    (:`Update`
      (`SceneComponent.K2_AddLocalOffset` (`self.StaticMesh`) (`KismetMathLibrary.VLerp` (0.0 0.0 0.0) (0.0 0.0 5.0) _float) false false))
    (:`Finished`
      (`PrimitiveComponent.SetCollisionEnabled` (`self.StaticMesh`) "NoCollision")
      (`self.K2_DestroyActor`))))

(fn `UserConstructionScript`
  (`StaticMeshComponent.SetStaticMesh` (`self.StaticMesh`) (`self.StoneMesh`)))