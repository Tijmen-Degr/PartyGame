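; BP_ClimbPlayer is the player character for the ClimbTheWall level, scaled up on BeginPlay and driven by the W key.
; Each press reads the climb stage from AnimBP_Climb, raises its CanJump flag, then after a timed delay advances the stage and clears the flag.
; The second stage also teleports the actor to a fixed ledge position; a smoothed timeline move is left disabled.
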(event `self.ReceiveBeginPlay`
  (`self.SetActorScale3D` (1.5 1.5 1.5)))

(event `Key|W`
  (params (Key :type "Key Structure"))
  (:`Pressed`
    (bind _asanim_bp_climb (cast `/Game/Levels/ClimbTheWall/AnimBP_Climb` (`SkeletalMeshComponent.GetAnimInstance` (`self.Mesh`))))
    (switch `int` (`/Game/Levels/ClimbTheWall/AnimBP_Climb.CurrentStage` _asanim_bp_climb)
      (:`0`
        (set `/Game/Levels/ClimbTheWall/AnimBP_Climb.CanJump` true _asanim_bp_climb)
        (`KismetSystemLibrary.Delay` 1.0)
        (set `/Game/Levels/ClimbTheWall/AnimBP_Climb.CurrentStage` 1 _asanim_bp_climb)
        (set `/Game/Levels/ClimbTheWall/AnimBP_Climb.CanJump` false _asanim_bp_climb))
      (:`1`
        (set `/Game/Levels/ClimbTheWall/AnimBP_Climb.CanJump` true _asanim_bp_climb)
        (`KismetSystemLibrary.Delay` 1.73)
        (`self.K2_SetActorLocation` (600.0 100.0 425.0))
        (set `/Game/Levels/ClimbTheWall/AnimBP_Climb.CurrentStage` 2 _asanim_bp_climb)
        (set `/Game/Levels/ClimbTheWall/AnimBP_Climb.CanJump` false _asanim_bp_climb)))))

(fn `UserConstructionScript`)