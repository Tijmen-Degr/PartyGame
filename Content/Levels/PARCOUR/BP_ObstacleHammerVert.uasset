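; Vertical swinging hammer obstacle for the parkour level that knocks the player character into a ragdoll on impact.
; Any hit on its static mesh plays a 2D ricochet sound, then only a BP_Parcour_character gets ragdolled.
; The launch vector follows the hit's normal impulse direction, scaled by the absolute swing speed read from BPAngleRotator, with a minimum upward component so victims are always thrown up.
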(event `self.StaticMeshComponent.OnComponentHit`
  (params (HitComponent :type "PrimitiveComponent Object Reference") (OtherActor :type "Actor Object Reference") (OtherComp :type "PrimitiveComponent Object Reference") (NormalImpulse :type "Vector Structure") (Hit :type "HitResult Structure (by ref)"))
  (`GameplayStatics.PlaySound2D` "/Game/VFX-SFX/vanoss-ricochet.vanoss-ricochet" 1.0 1.0 0.15 null null false)
  (bind _asbp_parcour_character (cast `/Game/Levels/PARCOUR/BP_Parcour_character` OtherActor))
  (`/Game/Levels/PARCOUR/BP_Parcour_character.Ragdoll` _asbp_parcour_character (`KismetMathLibrary.MakeVector` (.x (* (* (`KismetMathLibrary.Abs` (`/Game/Environments/Platformer_8_Underworld/Blueprints/Components/BP_AngleRotator.CurrentSwingSpeed` (`self.BP_AngleRotator`))) 1000.0) (`KismetMathLibrary.Normal` NormalImpulse))) (.y (* (* (`KismetMathLibrary.Abs` (`/Game/Environments/Platformer_8_Underworld/Blueprints/Components/BP_AngleRotator.CurrentSwingSpeed` (`self.BP_AngleRotator`))) 1000.0) (`KismetMathLibrary.Normal` NormalImpulse))) (`KismetMathLibrary.FMax` (.z (* (* (`KismetMathLibrary.Abs` (`/Game/Environments/Platformer_8_Underworld/Blueprints/Components/BP_AngleRotator.CurrentSwingSpeed` (`self.BP_AngleRotator`))) 1000.0) (`KismetMathLibrary.Normal` NormalImpulse))) 10000.0))))

(fn `UserConstructionScript`)