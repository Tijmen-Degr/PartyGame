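; Spinning obstacle for the parkour level that knocks the player into a ragdoll on contact.
; Any hit on its static mesh plays a cartoon slap sound, then only parkour characters are ragdolled.
; The launch vector follows the normalized hit impulse, scaled by the absolute rotation speed of its BPRotator, with a minimum upward component so victims always get thrown into the air.
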(event `self.StaticMeshComponent.OnComponentHit`
  (params (HitComponent :type "PrimitiveComponent Object Reference") (OtherActor :type "Actor Object Reference") (OtherComp :type "PrimitiveComponent Object Reference") (NormalImpulse :type "Vector Structure") (Hit :type "HitResult Structure (by ref)"))
  (`GameplayStatics.PlaySound2D` "/Game/VFX-SFX/floraphonic-cartoon-slap-1-189830.floraphonic-cartoon-slap-1-189830" 1.0 1.0 0.15 null null false)
  (bind _asbp_parcour_character (cast `/Game/Levels/PARCOUR/BP_Parcour_character` OtherActor))
  (`/Game/Levels/PARCOUR/BP_Parcour_character.Ragdoll` _asbp_parcour_character (`KismetMathLibrary.MakeVector` (.x (* (`KismetMathLibrary.Abs` (`/Game/Environments/Platformer_8_Underworld/Blueprints/Components/BP_Rotator.RotationSpeed` (`self.BP_Rotator`))) (`KismetMathLibrary.Normal` NormalImpulse))) (.y (* (`KismetMathLibrary.Abs` (`/Game/Environments/Platformer_8_Underworld/Blueprints/Components/BP_Rotator.RotationSpeed` (`self.BP_Rotator`))) (`KismetMathLibrary.Normal` NormalImpulse))) (`KismetMathLibrary.FMax` (.z (* (`KismetMathLibrary.Abs` (`/Game/Environments/Platformer_8_Underworld/Blueprints/Components/BP_Rotator.RotationSpeed` (`self.BP_Rotator`))) (`KismetMathLibrary.Normal` NormalImpulse))) 1000.0))))

(fn `UserConstructionScript`)