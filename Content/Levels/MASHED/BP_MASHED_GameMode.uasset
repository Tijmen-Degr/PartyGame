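; Game mode for the MASHED level that manages local multiplayer players and respawns the parkour character.
; A one-second looping timer compares local player count to connected input devices minus one (minimum one), creating or removing players until they match.
; The skip-gamepad-to-player-1 setting forces the target to one.
; RespawnPLayer waits briefly, spawns at LastCheckpoint or the supplied transform, and possesses only with player controller 0.
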(event `self.ReceiveBeginPlay`
  (bind _returnvalue (`GameplayStatics.GetNumLocalPlayerControllers`))
  (`KismetSystemLibrary.K2_SetTimerDelegate` (delegate `CheckControllers`) 1.0 true)
  (bind (_outinputdevices _returnvalue_2) (`InputDeviceLibrary.GetAllConnectedInputDevices` :!label _label))
  (bind _returnvalue_3 (`KismetMathLibrary.Max` (select `bool` (`GameMapsSettings.GetSkipAssigningGamepadToPlayer1` (`GameMapsSettings.GetGameMapsSettings`)) :`false` (- _returnvalue_2 1)) 1))
  (if (> _returnvalue_3 _returnvalue)
    (`GameplayStatics.CreatePlayer` _returnvalue)
    (goto _label)
    (elif (< _returnvalue_3 _returnvalue)
      (`GameplayStatics.RemovePlayer` (`GameplayStatics.GetPlayerController` (- _returnvalue 1)) true)
      (goto _label))))

(event `CheckControllers`
  (goto _label))

(event `RespawnPLayer`
  (params (SpawnTransform :type "Transform Structure"))
  (bind _returnvalue (`GameplayStatics.GetPlayerController` 0))
  (`KismetSystemLibrary.Delay` 1.5)
  (bind _last_checkpoint (`self.Last Checkpoint`)
    (:`then`
      (bind _returnvalue_location (`KismetMathLibrary.BreakTransform` (`SceneComponent.K2_GetComponentToWorld` (`/Game/Levels/PARCOUR/BP_CheckpointGate.POS` _last_checkpoint))))
      (bind _returnvalue_2 (`|SpawnActorFromClass` "/Game/Levels/PARCOUR/BP_Parcour_character.BP_Parcour_character_C" (`KismetMathLibrary.MakeTransform` _returnvalue_location (struct :`Yaw` 90.0)) "AlwaysSpawn" "MultiplyWithRoot" null null))
      (`Controller.Possess` _returnvalue _returnvalue_2))
    (:`else`
      (bind _returnvalue_3 (`|SpawnActorFromClass` "/Game/Levels/PARCOUR/BP_Parcour_character.BP_Parcour_character_C" SpawnTransform "Undefined" "MultiplyWithRoot" null null))
      (`Controller.Possess` _returnvalue _returnvalue_3))))

(fn `UserConstructionScript`)