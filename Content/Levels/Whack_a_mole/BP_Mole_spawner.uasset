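; Mole hole spawner for the Whack-a-mole level that keeps at most one tracked BP_Mole at its own location.
; BeginPlay starts a looping timer on StartSpawning, with an interval randomized once per spawner.
; StartSpawning spawns only when CurrentMole is invalid, then re-checks after a short delay.
; SpawnMole sets CurrentMole from the last GetAllActorsOfClass result; the random-area placement nodes and removal callback are unused or empty.
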(event `StartSpawning`
  ; Spawn mole logic (also checks if mole is already at a hole before spawning a new mole)
  (if (not (`KismetSystemLibrary.IsValid` (`self.CurrentMole`)))
    (`self.SpawnMole`)
    (`KismetSystemLibrary.Delay` 1.0)
    (`self.StartSpawning`)))

(event `self.ReceiveBeginPlay`
  ; Starts spawning mole after a 5 second countdown
  (`KismetSystemLibrary.K2_SetTimer` null "StartSpawning" (`KismetMathLibrary.RandomFloatInRange` 3.0 8.0) true))

(fn `OnMoleRemovedCallback`)

(fn `SpawnMole`
  (`|SpawnActorFromClass` "/Game/Levels/Whack_a_mole/BP_Mole.BP_Mole_C" (`KismetMathLibrary.MakeTransform` (`KismetMathLibrary.MakeVector` (.x (`self.K2_GetActorLocation`)) (.y (`self.K2_GetActorLocation`)) (.z (`self.K2_GetActorLocation`)))) "AdjustIfPossibleButAlwaysSpawn" "MultiplyWithRoot" null null)
  (bind _outactors (`GameplayStatics.GetAllActorsOfClass` "/Game/Levels/Whack_a_mole/BP_Mole.BP_Mole_C"))
  (set `self.CurrentMole` (`|GetArrayItem` _outactors (`KismetArrayLibrary.Array_LastIndex` _outactors))))

(fn `UserConstructionScript`)