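; BP_Mole is a mole actor for the Whack-a-mole level that pops up once and then removes itself.
; On BeginPlay it gives itself a random yaw and picks a random mesh from MoleMeshes for the MoleList component.
; A Rise timeline and then a Lowering timeline drive that component's relative location, and the actor is destroyed when lowering finishes.
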(event `self.ReceiveBeginPlay`
  (bind _mole_meshes (`self.Mole meshes`))
  ; On mole spawn set random rotation, set random mole and play up and down animation
  (`self.K2_SetActorRotation` (`KismetMathLibrary.MakeRotator` 0.0 0.0 (`KismetMathLibrary.RandomFloatInRange` 50.0 360.0)))
  (bind _output_get (set `self.CurrentMoleIndex` (`KismetMathLibrary.RandomIntegerInRange` 0 (- (`KismetArrayLibrary.Array_Length` _mole_meshes) 1))))
  (`StaticMeshComponent.SetStaticMesh` (`self.MoleList`) (`|GetArrayItem` _mole_meshes _output_get))
  (bind (_direction _risingmole) (`Timeline|Rise`)
    (:`Update`
      (`SceneComponent.K2_SetRelativeLocation` (`self.MoleList`) _risingmole false false))
    (:`Finished`
      (bind (_direction_2 _risingmole_2) (`Timeline|Lowering`)
        (:`Update`
          (`SceneComponent.K2_SetRelativeLocation` (`self.MoleList`) _risingmole_2 false false))
        (:`Finished`
          (`self.K2_DestroyActor`))))))

(fn `UserConstructionScript`)