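; Car spawner for the Avalanche level that repeatedly spawns BP_Car_16 at its own location with a fixed rotation.
; BeginPlay starts a looping timer with a random 3–7 second period on StartSpawning, which also re-calls itself after a random delay, so the two triggers overlap.
; Mole-spawner leftovers remain: CurrentCar is set to the last BP_Mole found, not the spawned car, alongside an empty callback and unused random-area nodes.
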(event `StartSpawning`
  ; Spawn mole logic (also checks if car is already at )
  (`self.SpawnCar`)
  (`KismetSystemLibrary.Delay` (`KismetMathLibrary.RandomFloatInRange` 3.0 7.0))
  (`self.StartSpawning`))

(event `self.ReceiveBeginPlay`
  ; Starts spawning mole after a 5 second countdown
  (`KismetSystemLibrary.K2_SetTimer` null "StartSpawning" (`KismetMathLibrary.RandomFloatInRange` 3.0 7.0) true))

(fn `OnMoleRemovedCallback`)

(fn `SpawnCar`
  (`|SpawnActorFromClass` "/Game/Levels/Avalanche/Actors/BP_Car_16.BP_Car_16_C" (`KismetMathLibrary.MakeTransform` (`KismetMathLibrary.MakeVector` (.x (`self.K2_GetActorLocation`)) (.y (`self.K2_GetActorLocation`)) (.z (`self.K2_GetActorLocation`))) (struct :`Yaw` 90.0)) "AdjustIfPossibleButAlwaysSpawn" "MultiplyWithRoot" null null)
  (bind _outactors (`GameplayStatics.GetAllActorsOfClass` "/Game/Levels/Whack_a_mole/BP_Mole.BP_Mole_C"))
  (set `self.CurrentCar` (`|GetArrayItem` _outactors (`KismetArrayLibrary.Array_LastIndex` _outactors))))

(fn `UserConstructionScript`)