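; Game mode for the Avalanche level that provides logic to spawn or respawn a player's character.
; SpawnPlayer destroys the controller's current pawn, spawns BP_Avalanche_character at the transform from PlayerSpawn and possesses it.
; PlayerSpawn indexes all PlayerStart actors with a random integer, but its Min and Max are reversed (last index to zero).
; The event graph is empty, so nothing here calls SpawnPlayer.
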(fn `Player_spawn`
  (returns (Player_start_transform :type "Transform Structure (by ref)"))
  (bind _outactors (`GameplayStatics.GetAllActorsOfClass` "/Script/Engine.PlayerStart"))
  (return (`self.GetTransform` (`|GetArrayItem` _outactors (`KismetMathLibrary.RandomIntegerInRange` (- (`KismetArrayLibrary.Array_Length` _outactors) 1))))))

(fn `Spawn_player`
  (params (Player_controller :type "PlayerController Object Reference"))
  (bind _returnvalue (`Controller.K2_GetPawn` Player_controller))
  (`/Engine/EditorBlueprintResources/StandardMacros.IsValid` _returnvalue
    (:`Is Valid`
      (`self.K2_DestroyActor` _returnvalue))
    (:`Is Not Valid`
      _))
  (bind _returnvalue_2 (`|SpawnActorFromClass` "/Game/Levels/Avalanche/BP_Avalanche_character.BP_Avalanche_character_C" (`self.Player_spawn`) "Undefined" "MultiplyWithRoot" null null))
  (`Controller.Possess` Player_controller _returnvalue_2))

(fn `UserConstructionScript`)