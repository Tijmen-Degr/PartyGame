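; Van spawner for the Avalanche level that repeatedly spawns BP_Van at its own location with a fixed rotation.
; BeginPlay starts a looping timer on StartSpawning, with its interval randomized once.
; StartSpawning spawns a van and also re-calls itself after a random delay, so spawns come from both timer and self-loop.
; Random-in-box placement and car lookup logic are unused, and OnMoleRemovedCallback is empty.
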(event `StartSpawning`
  ; Spawn car logic (also checks if car is already at )
  (`self.SpawnCar`)
  (`KismetSystemLibrary.Delay` (`KismetMathLibrary.RandomFloatInRange` 3.0 7.0))
  (`self.StartSpawning`))

(event `self.ReceiveBeginPlay`
  ; Starts spawning car after a 5 second countdown
  (`KismetSystemLibrary.K2_SetTimer` null "StartSpawning" (`KismetMathLibrary.RandomFloatInRange` 3.0 7.0) true))

(fn `OnMoleRemovedCallback`)

(fn `SpawnCar`
  (`|SpawnActorFromClass` "/Game/Levels/Avalanche/Actors/BP_Van.BP_Van_C" (`KismetMathLibrary.MakeTransform` (`KismetMathLibrary.MakeVector` (.x (`self.K2_GetActorLocation`)) (.y (`self.K2_GetActorLocation`)) (.z (`self.K2_GetActorLocation`))) (struct :`Yaw` 90.0)) "AdjustIfPossibleButAlwaysSpawn" "MultiplyWithRoot" null null))

(fn `UserConstructionScript`)