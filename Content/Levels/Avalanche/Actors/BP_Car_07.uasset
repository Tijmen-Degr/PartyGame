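; BP_Car_07 is a physics-driven car hazard in the Avalanche level that ragdolls any BP_Avalanche_character it hits.
; BeginPlay launches the mesh along negative X and downward with a velocity-change impulse, then starts a looping Accelerate timer with a randomized interval.
; Accelerate re-pushes the car and also re-calls itself after a random delay, or gives a weaker push with a debug print when stationary.
; A GameStarted check is left unconnected.
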(event `ApplySpeed`
  (`PrimitiveComponent.AddImpulse` (`self.StaticMesh`) (-2000.0 0.0 -1500.0) "None" true))

(event `Accelerate`
  (if (> (`KismetMathLibrary.VSize` (`self.GetVelocity`)) 0.0)
    (`self.ApplySpeed`)
    (`KismetSystemLibrary.Delay` (`KismetMathLibrary.RandomFloatInRange` 4.0 6.0))
    (`self.Accelerate`)
    (else
      (`KismetSystemLibrary.PrintString` "no vroom vroom")
      (`PrimitiveComponent.AddImpulse` (`self.StaticMesh`) (-1000.0 0.0 -1500.0) "None" true))))

(event `self.ReceiveBeginPlay`
  (`PrimitiveComponent.AddImpulse` (`self.StaticMesh`) (-5000.0 0.0 -1000.0) "None" true)
  (`KismetSystemLibrary.K2_SetTimer` null "Accelerate" (`KismetMathLibrary.RandomFloatInRange` 4.0 6.0) true))

(event `self.ReceiveHit`
  (params (MyComp :type "PrimitiveComponent Object Reference") (Other :type "Actor Object Reference") (OtherComp :type "PrimitiveComponent Object Reference") (bSelfMoved :type Boolean) (HitLocation :type "Vector Structure") (HitNormal :type "Vector Structure") (NormalImpulse :type "Vector Structure") (Hit :type "HitResult Structure (by ref)"))
  (bind _asbp_avalanche_character (cast `/Game/Levels/Avalanche/BP_Avalanche_character` Other))
  (`/Game/Levels/Avalanche/BP_Avalanche_character.Ragdoll` _asbp_avalanche_character))

(fn `UserConstructionScript`)