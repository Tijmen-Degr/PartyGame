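; BP_Car_meshes is a physics-driven car hazard in the Avalanche level that ragdolls the Avalanche character on hit.
; BeginPlay picks a random mesh from CarMeshes and launches it with a velocity-change impulse toward negative X and downward.
; A looping timer, alongside Accelerate's delayed self-call, repeats the push at randomized intervals.
; Accelerate destroys the actor if it finds it has stopped moving.
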(event `SpeedApply`
  (`PrimitiveComponent.AddImpulse` (`self.StaticMesh`) (-2000.0 0.0 -1500.0) "None" true))

(event `Accelerate`
  (if (> (`KismetMathLibrary.VSize` (`self.GetVelocity`)) 0.0)
    (`self.SpeedApply`)
    (`KismetSystemLibrary.Delay` (`KismetMathLibrary.RandomFloatInRange` 4.0 6.0))
    (`self.Accelerate`)
    (else
      (`KismetSystemLibrary.PrintString` "no vroom vroom")
      (`self.K2_DestroyActor`))))

(event `self.ReceiveBeginPlay`
  (bind _car_meshes (`self.Car_meshes`))
  (`StaticMeshComponent.SetStaticMesh` (`self.StaticMesh`) (`|GetArrayItem` _car_meshes (`KismetMathLibrary.RandomIntegerInRange` 0 (- (`KismetArrayLibrary.Array_Length` _car_meshes) 1))))
  (`PrimitiveComponent.AddImpulse` (`self.StaticMesh`) (-5000.0 0.0 -600.0) "None" true)
  (`KismetSystemLibrary.K2_SetTimer` null "Accelerate" (`KismetMathLibrary.RandomFloatInRange` 4.0 6.0) true))

(event `self.StaticMesh.OnComponentHit`
  (params (HitComponent :type "PrimitiveComponent Object Reference") (OtherActor :type "Actor Object Reference") (OtherComp :type "PrimitiveComponent Object Reference") (NormalImpulse :type "Vector Structure") (Hit :type "HitResult Structure (by ref)"))
  (bind _asbp_avalanche_character (cast `/Game/Levels/Avalanche/BP_Avalanche_character` OtherActor))
  (`/Game/Levels/Avalanche/BP_Avalanche_character.Ragdoll` _asbp_avalanche_character))

(fn `UserConstructionScript`)